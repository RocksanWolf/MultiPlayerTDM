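; Base character Blueprint that handles picking up weapons the character walks over.
; Capsule overlaps with BP_WeaponBaseClass actors store the weapon and toggle a CanPickup flag.
; PickupWeapon casts the stored weapon to pistol or rifle and passes that type to TakeWeapon.
; TakeWeapon snaps a pistol to the mesh's WeaponSocket unless HasPistol is set; rifles have no attach logic yet.
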(event `self.CapsuleComponent.OnComponentBeginOverlap`
  (params (OverlappedComponent :type "PrimitiveComponent Object Reference") (OtherActor :type "Actor Object Reference") (OtherComp :type "PrimitiveComponent Object Reference") (OtherBodyIndex :type Integer) (bFromSweep :type Boolean) (SweepResult :type "HitResult Structure (by ref)"))
  ;[1 1 1] Check if i can pickup weapon'
  (bind _asbp_weapon_base_class (cast `/Game/Blueprint/Weapons/BP_WeaponBaseClass` OtherActor))
  (set `self.Weapon` _asbp_weapon_base_class)
  (set `self.CanPickup?` true))

(event `self.CapsuleComponent.OnComponentEndOverlap`
  (params (OverlappedComponent :type "PrimitiveComponent Object Reference") (OtherActor :type "Actor Object Reference") (OtherComp :type "PrimitiveComponent Object Reference") (OtherBodyIndex :type Integer))
  ;[1 1 1] Check if i can pickup weapon'
  (cast `/Game/Blueprint/Weapons/BP_WeaponBaseClass` OtherActor)
  (set `self.CanPickup?` false))

(event `PickupWeapon`
  (bind _weapon (`self.Weapon`))
  ;[1 1 1] Pickup Event
  (if (`self.CanPickup?`)
    (bind _asbp_pistol (cast `/Game/Blueprint/Weapons/Pistol/BP_Pistol` _weapon)
      (:`then`
        (set `self.Pistol` _asbp_pistol)
        (`self.TakeWeapon` "NewEnumerator0"))
      (:`CastFailed`
        (bind _asbp_rifle (cast `/Game/Blueprint/Weapons/Rifle/BP_Rifle` _weapon))
        (set `self.Rifle` _asbp_rifle)
        (`self.TakeWeapon` "NewEnumerator1")))))

(event `TakeWeapon`
  (params (WeaponList :type "/Game/Blueprint/Enumerations/BP_WeaponsListEnum Enum" :default "NewEnumerator0"))
  (bind _output_get (set `self.WeaponList` WeaponList))
  (switch `/Game/Blueprint/Enumerations/BP_WeaponsListEnum` _output_get
    (:`NewEnumerator0`
      (if (not (`self.HasPistol`))
        (`SceneComponent.K2_AttachToComponent` (`Actor.RootComponent` (`self.Pistol`)) (`self.Mesh`) "WeaponSocket" "SnapToTarget" "SnapToTarget" "SnapToTarget" true)))))

(fn `UserConstructionScript`)