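; Base player character Blueprint that turns player input into movement, camera look and weapon actions.
; Axis inputs feed movement along the actor's forward and right vectors, plus controller yaw and pitch.
; Action presses trigger jumping or delegate to weapon pickup, pistol and rifle equip, and shooting functions, whose logic lives outside these graphs.
; The construction script only calls its parent.
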(event `InputAxis|MoveForward`
  (params (AxisValue :type "Float (single-precision)"))
  ;[1 1 1] Character Movement
  (`self.AddMovementInput` (`self.GetActorForwardVector`) AxisValue))

(event `InputAction|Pickup`
  (params (Key :type "Key Structure"))
  ;[1 1 1] Pickup weapon if key pressed
  (:`Pressed`
    (`self. PickupWeapon`)))

(event `InputAxis|MoveRight`
  (params (AxisValue :type "Float (single-precision)"))
  ;[1 1 1] Character Movement
  (`self.AddMovementInput` (`self.GetActorRightVector`) AxisValue))

(event `InputAction|PistolEquip`
  (params (Key :type "Key Structure"))
  ;[1 1 1] Equip/Unequip Weapon
  (:`Pressed`
    (`self.EquipPistol`)))

(event `InputAxis|LookAround`
  (params (AxisValue :type "Float (single-precision)"))
  ;[1 1 1] Character Movement
  (`self.AddControllerYawInput` AxisValue))

(event `InputAction|RifleEquip`
  (params (Key :type "Key Structure"))
  ;[1 1 1] Equip/Unequip Weapon
  (:`Pressed`
    (`self.EquipRifle`)))

(event `InputAxis|LookUpDown`
  (params (AxisValue :type "Float (single-precision)"))
  ;[1 1 1] Character Movement
  (`self.AddControllerPitchInput` AxisValue))

(event `InputAction|Fire`
  (params (Key :type "Key Structure"))
  ;[1 1 1] Fire
  (:`Pressed`
    (`self.Shoot`)))

(event `InputAction|Jump`
  (params (Key :type "Key Structure"))
  ;[1 1 1] Character Movement
  (:`Pressed`
    (`self.Jump`)))

(fn `UserConstructionScript`
  (`parent.UserConstructionScript`))