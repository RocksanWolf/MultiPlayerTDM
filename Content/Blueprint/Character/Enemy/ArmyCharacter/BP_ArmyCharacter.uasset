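; BP_ArmyCharacter is an army enemy character that displays its health through an EnemyInfo widget component.
; On BeginPlay it runs the parent logic, creates a BP_EnemyHealthInfo widget, assigns it to EnemyInfo and fills the health bar from CurrentHealth on a fixed 100-point scale.
; A custom event reassigns the stored widget, refreshes the bar and hides EnemyInfo once health reaches zero or below.
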(event `self.ReceiveBeginPlay`
  (`parent.ReceiveBeginPlay`)
  (bind _returnvalue (`|CreateWidget` "/Game/Blueprint/UI/BP_EnemyHealthInfo.BP_EnemyHealthInfo_C"))
  (set `self.WidgetInfo` _returnvalue)
  (`WidgetComponent.SetWidget` (`self.EnemyInfo`) _returnvalue)
  (`ProgressBar.SetPercent` (`/Game/Blueprint/UI/BP_EnemyHealthInfo.HealthBar` _returnvalue) (/ (`self.CurrentHealth`) 100.0)))

(event `CustomEvent`
  (bind _currenthealth (`self.CurrentHealth`))
  (bind _widgetinfo (`self.WidgetInfo`))
  (`WidgetComponent.SetWidget` (`self.EnemyInfo`) _widgetinfo)
  (`ProgressBar.SetPercent` (`/Game/Blueprint/UI/BP_EnemyHealthInfo.HealthBar` _widgetinfo) (/ _currenthealth 100.0))
  (if (<= _currenthealth 0.0)
    (`SceneComponent.SetVisibility` (`self.EnemyInfo`) false false)))

(fn `UserConstructionScript`
  (`parent.UserConstructionScript`))