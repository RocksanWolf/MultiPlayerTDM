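; Base weapon Blueprint whose Shoot event fires a hitscan shot using the passed weapon's WeaponInfo.
; It spawns muzzle flash and sound at the Muzzle, then multi-line traces from the owning pawn's controller viewpoint.
; The trace end is the view's forward vector times BulletRange, without adding the start location.
; A successful trace spawns impact effect and sound at the first hit; no damage is applied.
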(event `Shoot`
  (params (WeaponType :type "/Game/Blueprint/Weapons/BP_WeaponBaseClass Object Reference"))
  (bind _weapontype (`self.WeaponType`))
  (bind _muzzle (`/Game/Blueprint/Weapons/BP_WeaponBaseClass.Muzzle` _weapontype))
  (bind (_weaponinfo_muzzleflash _weaponinfo_muzzlesoundeffect) (break `/Game/Blueprint/Structure/BP_WeaponInfo` (`/Game/Blueprint/Weapons/BP_WeaponBaseClass.WeaponInfo` _weapontype)))
  (bind (_weaponinfo_muzzleflash_2 _weaponinfo_muzzlesoundeffect_2 _weaponinfo_impacteffect _weaponinfo_impactsound _weaponinfo_bulletrange) (break `/Game/Blueprint/Structure/BP_WeaponInfo` (`/Game/Blueprint/Weapons/BP_WeaponBaseClass.WeaponInfo` (`self.WeaponType`))))
  (bind (_weaponinfo_muzzleflash_3 _weaponinfo_muzzlesoundeffect_3 _weaponinfo_impacteffect_2 _weaponinfo_impactsound_2) (break `/Game/Blueprint/Structure/BP_WeaponInfo` (`/Game/Blueprint/Weapons/BP_WeaponBaseClass.WeaponInfo` (`self.WeaponType`))))
  (bind _returnvalue (`SceneComponent.K2_GetComponentLocation` _muzzle))
  (set `self.WeaponType` WeaponType)
  (`GameplayStatics.SpawnEmitterAtLocation` _weaponinfo_muzzleflash _returnvalue (`SceneComponent.K2_GetComponentRotation` _muzzle))
  (`GameplayStatics.SpawnSoundAtLocation` _weaponinfo_muzzlesoundeffect _returnvalue (struct) 1.0 1.0 0.0 null null)
  (bind _aspawn (cast `Pawn` (`self.GetOwner` (`self.WeaponType`))))
  (bind _returnvalue_2 (`Pawn.GetController` _aspawn))
  (`/Engine/EditorBlueprintResources/StandardMacros.IsValid` _returnvalue_2
    (:`Is Valid`
      (bind (_location _rotation) (`Controller.GetPlayerViewPoint` _returnvalue_2))
      (bind _output_get (set `self.Location` _location))
      (set `self.Rotation` _rotation)
      (bind _output_get_2 (set `self.EndLocation` (* (`KismetMathLibrary.GetForwardVector` _rotation) _weaponinfo_bulletrange)))
      (bind (_outhits _returnvalue_3) (`KismetSystemLibrary.LineTraceMulti` _output_get _output_get_2 "TraceTypeQuery3"))
      (bind _output_get_3 (set `self.Out Hits` _outhits))
      (if _returnvalue_3
        (bind (_bblockinghit _binitialoverlap _time _distance _location_2) (`GameplayStatics.BreakHitResult` (`|GetArrayItem` _output_get_3)))
        (`GameplayStatics.SpawnEmitterAtLocation` _weaponinfo_impacteffect_2 _location_2)
        (`GameplayStatics.SpawnSoundAtLocation` _weaponinfo_impactsound_2 _location_2 (struct) 1.0 1.0 0.0 null null)))))

(fn `UserConstructionScript`)